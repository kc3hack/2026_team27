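; Ice block actor that shrinks in steps when something overlaps its MeltZone component.
; Each accepted overlap captures the IceBlock's world scale, and the Melting timeline lerps it to a uniformly smaller scale by a fixed step.
; A DoOnce ignores further overlaps until the timeline finishes, then resets so a new overlap can shrink it again.
; The overlapping actor is not filtered and the scale has no lower limit.
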(event OnComponentBeginOverlap(MeltZone)
  (params (OverlappedComponent :type Primitive%20Component%20Object%20Reference) (OtherActor :type Actor%20Object%20Reference) (OtherComp :type Primitive%20Component%20Object%20Reference) (OtherBodyIndex :type Integer) (bFromSweep :type Boolean) (SweepResult :type Hit%20Result%20Structure%20%28by%20ref%29))
  (bind _ice_block (Variables|Default|GetIce_Block))
  (Utilities|FlowControl|DoOnce false :!label _label
    (:Completed
      (bind _output_get (Variables|Default|SetStartScale (Transformation|GetWorldScale _ice_block)))
      (Variables|Default|SetTargetScale (- _output_get "0.100000,0.100000,0.100000"))
      (bind _alpha (Timeline|Melting PlayFromStart)
        (:Update
          (Transformation|SetWorldScale3D _ice_block (Math|Vector|Lerp(Vector) (Variables|Default|GetStartScale) (Variables|Default|GetTargetScale) _alpha)))
        (:Finished
          (goto _label Reset))))))

(event EventBeginPlay)

(event Collision|EventActorBeginOverlap
  (params (OtherActor :type Actor%20Object%20Reference)))

(event EventTick
  (params (DeltaSeconds :type Float%20%28single-precision%29)))

(fn ConstructionScript)