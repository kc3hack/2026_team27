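; Child fire effect Blueprint that plays Niagara fire and sound, then weakens when a combat character touches it.
; ActivateFireEvent starts both components.
; DamageFrag overlaps from BP_CombatCharacter lower CurrentFireScale one clamped step through the FadeOutFire timeline, which lerps both Niagara FireScale and sound volume.
; A DoOnce blocks further reductions until each fade finishes, so the fire dies down gradually over repeated overlaps.
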(event OnComponentBeginOverlap(DamageFrag)
  (params (OverlappedComponent :type Primitive%20Component%20Object%20Reference) (OtherActor :type Actor%20Object%20Reference) (OtherComp :type Primitive%20Component%20Object%20Reference) (OtherBodyIndex :type Integer) (bFromSweep :type Boolean) (SweepResult :type Hit%20Result%20Structure%20%28by%20ref%29))
  (Utilities|Casting|CastToBP_CombatCharacter OtherActor)
  (Utilities|FlowControl|DoOnce false :!label _label
    (:Completed
      (Variables|Default|SetStartScale (Variables|Default|GetCurrentFireScale))
      (Variables|Default|SetTargetScale (Math|Float|Clamp(Float) (- (Variables|Default|GetCurrentFireScale) 0.1)))
      (bind _alpha (Timeline|FadeOutFire Play)
        (:Update
          (bind _output_get (Variables|Default|SetCurrentFireScale (Math|Float|Lerp (Variables|Default|GetStartScale) (Variables|Default|GetTargetScale) _alpha)))
          (Audio|Components|Audio|SetVolumeMultiplier (Variables|Default|GetSND_Fire) _output_get :!class /Script/Engine.AudioComponent)
          (Niagara|SetNiagaraVariable(Float) (Variables|Default|GetNS_Fire) "FireScale" _output_get))
        (:Finished
          (goto _label Reset))))))

(event Custom|ActivateFireEvent
  (Components|Activation|Activate (Variables|Default|GetSND_Fire) false)
  (Components|Activation|Activate (Variables|Default|GetNS_Fire) false))

(event EventBeginPlay
  (|CallParentFunction) ; このノードは無効になっているため呼び出せません。\n機能をビルドするにはピンをドラッグしてください。
)

(event Collision|EventActorBeginOverlap
  (params (OtherActor :type Actor%20Object%20Reference))
  (|CallParentFunction OtherActor) ; このノードは無効になっているため呼び出せません。\n機能をビルドするにはピンをドラッグしてください。
)

(event EventTick
  (params (DeltaSeconds :type Float%20%28single-precision%29))
  (|CallParentFunction DeltaSeconds) ; このノードは無効になっているため呼び出せません。\n機能をビルドするにはピンをドラッグしてください。
)

(fn ConstructionScript
  (|CallParentFunction))