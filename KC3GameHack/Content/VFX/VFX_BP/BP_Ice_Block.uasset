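; Ice block effect Blueprint that melts a little each time its TriggerEffectEvent fires.
; The event starts the audio, records the IceBlock component's world scale and sets a target slightly smaller on every axis by a fixed amount.
; The Melting timeline interpolates the scale down to that target, then stops the audio when finished.
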(event EventTriggerEffectEvent
  (bind _ice_block (Variables|Default|GetIce_Block))
  (Audio|Components|Audio|Play (Variables|Default|GetAudio) 0.0)
  (bind _output_get (Variables|Default|SetStartScale (Transformation|GetWorldScale _ice_block)))
  (Variables|Default|SetTargetScale (- _output_get "0.100000,0.100000,0.100000"))
  (bind _alpha (Timeline|Melting PlayFromStart)
    (:Update
      (Transformation|SetWorldScale3D _ice_block (Math|Vector|Lerp(Vector) (Variables|Default|GetStartScale) (Variables|Default|GetTargetScale) _alpha)))
    (:Finished
      (Audio|Components|Audio|Stop (Variables|Default|GetAudio)))))

(fn ConstructionScript)